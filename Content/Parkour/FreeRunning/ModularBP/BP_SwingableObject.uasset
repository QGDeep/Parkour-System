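; Swingable bar for the free-running parkour system, overriding a parent's construction to position hand IK points and drop the unneeded LandPosition component.
; GetLandPosition snaps HandIKRoot to the spline point closest to player 0 and returns it, so the grip follows the player along the bar.
; GetSwingDirectionAndIK tests front/back arrows against MinDot, returning swing validity, rotation and hand targets, swapped by side and offset against the facing direction.
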(fn `GetLandPosition`
  (returns (Location :type "Vector Structure"))
  (bind _returnvalue (`SplineComponent.FindLocationClosestToWorldLocation` (`self.Spline`) (`self.K2_GetActorLocation` (`GameplayStatics.GetPlayerCharacter` 0)) "World"))
  ;[0.03906 0.5024 1] Set the IK parent scene component so both move relative to it and return the players closest location to the spline
  (`SceneComponent.K2_SetWorldLocation` (`self.HandIKRoot`) _returnvalue false false)
  (return _returnvalue))

(fn `GetSwingDirectionAndIK`
  (params (MinDot :type "Float (double-precision)"))
  (returns (CanSwing :type Boolean) (LeftHandIK :type "Vector Structure") (RightHandIK :type "Vector Structure") (DirectionRotation :type "Rotator Structure"))
  (bind (_facing _facingarrow _isfrontarrow) (`self.FindFaceDirection` (`self.FrontArrow`) (`self.BackArrow`) MinDot))
  (bind _returnvalue (* (`KismetMathLibrary.NegateVector` (`SceneComponent.GetForwardVector` _facingarrow)) 8.0))
  ;[0.03906 0.5024 1] Find facing direction and find hand IK positions by using an offset
  (return _facing (+ (`SceneComponent.K2_GetComponentLocation` (select `bool` _isfrontarrow :`false` (`self.LeftHandIKPosition`) :`true` (`self.RightHandIKPosition`))) _returnvalue) (+ (`SceneComponent.K2_GetComponentLocation` (select `bool` _isfrontarrow :`false` (`self.RightHandIKPosition`) :`true` (`self.LeftHandIKPosition`))) _returnvalue) (`KismetMathLibrary.MakeRotFromX` (`SceneComponent.GetForwardVector` _facingarrow))))

(fn `GetType`
  (returns (Type :type "/Game/Parkour/FreeRunning/Enum_MoveableObjectType Enum"))
  (return "NewEnumerator2"))

(fn `UserConstructionScript`
  ;[0.03906 0.5024 1] Set hand Ik positions and destroy land position as it is not needed
  (`parent.UserConstructionScript`)
  (`SceneComponent.K2_SetRelativeLocation` (`self.LeftHandIKPosition`) (`self.LeftHandIKPos`) false false)
  (`SceneComponent.K2_SetRelativeLocation` (`self.RightHandIKPosition`) (`self.RightHandIKPos`) false false)
  (`ActorComponent.K2_DestroyComponent` (`self.LandPosition`)))