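; Spline-based parkour beam actor that supplies landing data for the player character.
; The construction script tiles spline meshes at fixed-length intervals with normalized tangents and uniform scale, optionally forcing every point to one spline type.
; Getters return the spline point closest to player 0 as the landing position, a raised midpoint between player and that point as the peak, plus the Beam type and a thin-object flag.
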(fn `GetLandPosition`
  (returns (Location :type "Vector Structure"))
  (return (`SplineComponent.FindLocationClosestToWorldLocation` (`self.Spline`) (`self.K2_GetActorLocation` (`GameplayStatics.GetPlayerCharacter` 0)) "World")))

(fn `GetPeakPosition`
  (returns (Location :type "Vector Structure"))
  (bind _returnvalue (`self.K2_GetActorLocation` (`GameplayStatics.GetPlayerCharacter` 0)))
  (bind (_returnvalue_x _returnvalue_y _returnvalue_z) (`KismetMathLibrary.BreakVector` (`KismetMathLibrary.GetVectorArrayAverage` (`|MakeArray` (`SplineComponent.FindLocationClosestToWorldLocation` (`self.Spline`) _returnvalue "World") _returnvalue))))
  ; Get the peak position by getting the closest position on the spline and adding a Z offset
  (return (`KismetMathLibrary.MakeVector` _returnvalue_x _returnvalue_y (+ _returnvalue_z 40.0))))

(fn `GetSpline`
  (returns (Spline :type "SplineComponent Object Reference"))
  (return null))

(fn `GetSplineStartAndEnd`
  (params (Index :type Integer))
  (returns (Location :type "Vector Structure") (Tangent :type "Vector Structure"))
  (bind _spline (`self.Spline`))
  (bind _returnvalue (* Index (`self.MeshLength`)))
  (return (`SplineComponent.GetLocationAtDistanceAlongSpline` _spline _returnvalue "Local") (`KismetMathLibrary.Normal` (`SplineComponent.GetTangentAtDistanceAlongSpline` _spline _returnvalue "Local"))))

(fn `GetType`
  (returns (Type :type "EMoveableObjectType Enum"))
  (return "Beam"))

(fn `IsThinObject`
  (returns (ReturnValue :type Boolean))
  (return (`self.ThinObject`)))

(fn `UserConstructionScript`
  (bind _meshscale (`self.MeshScale`))
  (bind _meshscale_2 (`self.MeshScale`))
  ;[0.9911 0.9911 0.9911] Add the spline mesh using a for loop. Set start and end points get the locations and tangents so it can be curved or straight (linear).
  (for _index (range (+ (`KismetMathLibrary.FTrunc` (/ (`SplineComponent.GetSplineLength` (`self.Spline`)) (`self.MeshLength`))) 1))
    (bind _returnvalue (`AddComponent|NODE_AddSplineMeshComponent-0` :`RelativeTransform` (`KismetMathLibrary.MakeTransform` (`KismetMathLibrary.MakeVector` 0.0 0.0 (`self.ZOffset`)))))
    (`StaticMeshComponent.SetStaticMesh` _returnvalue (`self.BeamMesh`))
    (`SceneComponent.K2_AttachToComponent` _returnvalue (`self.DefaultSceneRoot`) "None" "KeepRelative" "KeepRelative" "KeepRelative" true)
    (bind (_location _tangent) (`self.GetSplineStartAndEnd` _index))
    (bind (_location_2 _tangent_2) (`self.GetSplineStartAndEnd` (+ _index 1)))
    (`SplineMeshComponent.SetStartAndEnd` _returnvalue _location _tangent _location_2 _tangent_2 true)
    (set `SplineComponent.bInputSplinePointsToConstructionScript` true (`self.Spline`))
    (`SplineMeshComponent.SetStartScale` _returnvalue (`KismetMathLibrary.MakeVector2D` _meshscale _meshscale) true)
    (`SplineMeshComponent.SetEndScale` _returnvalue (`KismetMathLibrary.MakeVector2D` _meshscale_2 _meshscale_2) true)
    ;[0.4072 0.4072 0.4072] Set spline point type to linear or curved
    (if (`self.ForceSplinePointType`)
      (for _index_2 (range (`SplineComponent.GetNumberOfSplinePoints` (`self.Spline`)))
        (`SplineComponent.SetSplinePointType` (`self.Spline`) _index_2 (`self.SplineType`) true)))))